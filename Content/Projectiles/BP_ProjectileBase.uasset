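; Base projectile actor that flies with configurable speed and gravity, optionally homing on a target, and expires after its lifespan.
; The construction script copies speed, gravity and, for a valid target with homing enabled, homing settings into ProjectileMovement.
; Box overlaps ignore the owner and other projectiles.
; Other overlaps fire the OnProjectileImpact dispatcher, play impact effect and sound, damage any HealthComponent, then destroy the projectile.
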(event `self.ReceiveBeginPlay`
  (`self.SetLifeSpan` (`self.LifeSpan`)))

(event `self.Box.OnComponentBeginOverlap`
  (params (OverlappedComponent :type "PrimitiveComponent Object Reference") (OtherActor :type "Actor Object Reference") (OtherComp :type "PrimitiveComponent Object Reference") (OtherBodyIndex :type Integer) (bFromSweep :type Boolean) (SweepResult :type "HitResult Structure (by ref)"))
  (bind (_bblockinghit _binitialoverlap _time _distance _location) (`GameplayStatics.BreakHitResult` SweepResult))
  (bind _returnvalue (`self.GetComponentByClass` OtherActor "/Game/Characters/ActorComponents/HealthComponent.HealthComponent_C"))
  (if (not (== (`self.GetOwner`) OtherActor))
    (`KismetSystemLibrary.IsObjectOfSoftClass` OtherActor "/Game/Projectiles/BP_ProjectileBase.BP_ProjectileBase_C"
      (:`False`
        (`self.OnProjectileImpact` OtherActor SweepResult)
        (`GameplayStatics.SpawnEmitterAtLocation` (`self.Impact Effect`) _location)
        (`GameplayStatics.PlaySoundAtLocation` (`self.Sound`) _location (struct) 1.0 1.0 0.0 null null null null)
        (`/Engine/EditorBlueprintResources/StandardMacros.IsValid` _returnvalue
          (:`Is Valid`
            (`/Game/Characters/ActorComponents/HealthComponent.TakeDamage` _returnvalue (`self.Damage`)))
          (:`Is Not Valid`
            _))
        (`self.K2_DestroyActor`)))))

(fn `UserConstructionScript`
  (bind _projectilemovement (`self.ProjectileMovement`))
  (set `ProjectileMovementComponent.InitialSpeed` (`self.Speed`) _projectilemovement)
  (set `ProjectileMovementComponent.MaxSpeed` (`self.Speed`) _projectilemovement)
  (set `ProjectileMovementComponent.ProjectileGravityScale` (`self.Gravity`) _projectilemovement)
  (`self.Target`
    (:`then`
      (if (`self.IsHoming`)
        (set `ProjectileMovementComponent.bIsHomingProjectile` true _projectilemovement)
        (set `ProjectileMovementComponent.HomingAccelerationMagnitude` (`self.HomingAcceleration`) _projectilemovement)
        (set `ProjectileMovementComponent.HomingTargetComponent` (`Actor.RootComponent` (`self.Target`)) _projectilemovement)))
    (:`else`)))