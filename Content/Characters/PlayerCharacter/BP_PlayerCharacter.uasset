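; BP_PlayerCharacter is the player character Blueprint, with a simple projectile attack and damage feedback.
; A left mouse press spawns a short-lived homing BP_ProjectileBase at the Scene component's world transform, with the character as owner and instigator.
; The HealthComponent's OnDamageTaken event prints current health to the screen, while the construction script only calls its parent.
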(event `self.ReceiveBeginPlay`)

(event `self.HealthComponent.OnDamageTaken`
  (`KismetSystemLibrary.PrintString` (`KismetStringLibrary.Conv_DoubleToString` (`/Game/Characters/ActorComponents/HealthComponent.Health` (`self.HealthComponent`)))))

(event `Key|LeftMouseButton`
  (params (Key :type "Key Structure"))
  (:`Pressed`
    (`|SpawnActorFromClass` "/Game/Projectiles/BP_ProjectileBase.BP_ProjectileBase_C" (`SceneComponent.K2_GetComponentToWorld` (`self.Scene`)) "Undefined" "MultiplyWithRoot" self 2000.0 0.0 null true 2000.0 75.0 (0.0 0.0 0.0) 0.5 self)))

(fn `UserConstructionScript`
  (`parent.UserConstructionScript`))