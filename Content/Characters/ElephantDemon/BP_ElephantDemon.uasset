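; Elephant demon boss character that constantly turns toward the player and runs a repeating bullet-hell attack cycle from BeginPlay.
; BossFightLoop chains a timer-driven six-arm rotating spiral, radial projectile rings, a launched charge ending in another ring, and timed homing shots, all using BP_ProjectileCorona.
; Capsule hits deal massive damage to anything with a HealthComponent.
; Death is checked only at cycle end, either destroying the boss or restarting the loop.
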(event `RadialBurst`
  (params (Speed :type "Float (double-precision)") (Damage :type "Float (double-precision)"))
  (for _index (range 72)
    (`|SpawnActorFromClass` "/Game/Projectiles/BP_ProjectileCorona.BP_ProjectileCorona_C" (`KismetMathLibrary.MakeTransform` (- (`self.K2_GetActorLocation`) (0.0 0.0 250.0)) (`KismetMathLibrary.MakeRotator` 0.0 0.0 (`KismetMathLibrary.Conv_IntToDouble` (* _index 5)))) "Undefined" "MultiplyWithRoot" self Speed 0.0 null false 10000.0 Damage (0.0 0.0 0.0) 1.75 self)))

(event `SpiralSpurt`
  (`|SpawnActorFromClass` "/Game/Projectiles/BP_ProjectileCorona.BP_ProjectileCorona_C" (`KismetMathLibrary.MakeTransform` (- (`self.K2_GetActorLocation`) (0.0 0.0 250.0)) (`KismetMathLibrary.MakeRotator` 0.0 0.0 (`KismetMathLibrary.Conv_IntToDouble` (`KismetMathLibrary.FTrunc` (`self.SpiralOffset`))))) "Undefined" "MultiplyWithRoot" self (stale `SpiralFire` Speed) 0.0 null false 2000.0 (stale `SpiralFire` Damage) (0.0 0.0 0.0) 1.75 self)
  (`|SpawnActorFromClass` "/Game/Projectiles/BP_ProjectileCorona.BP_ProjectileCorona_C" (`KismetMathLibrary.MakeTransform` (- (`self.K2_GetActorLocation`) (0.0 0.0 250.0)) (`KismetMathLibrary.MakeRotator` 0.0 0.0 (`KismetMathLibrary.Conv_IntToDouble` (`KismetMathLibrary.FTrunc` (- (`self.SpiralOffset`) 60.0))))) "Undefined" "MultiplyWithRoot" self (stale `SpiralFire` Speed) 0.0 null false 2000.0 (stale `SpiralFire` Damage) (0.0 0.0 0.0) 1.75 self)
  (`|SpawnActorFromClass` "/Game/Projectiles/BP_ProjectileCorona.BP_ProjectileCorona_C" (`KismetMathLibrary.MakeTransform` (- (`self.K2_GetActorLocation`) (0.0 0.0 250.0)) (`KismetMathLibrary.MakeRotator` 0.0 0.0 (`KismetMathLibrary.Conv_IntToDouble` (`KismetMathLibrary.FTrunc` (- (`self.SpiralOffset`) 120.0))))) "Undefined" "MultiplyWithRoot" self (stale `SpiralFire` Speed) 0.0 null false 2000.0 (stale `SpiralFire` Damage) (0.0 0.0 0.0) 1.75 self)
  (`|SpawnActorFromClass` "/Game/Projectiles/BP_ProjectileCorona.BP_ProjectileCorona_C" (`KismetMathLibrary.MakeTransform` (- (`self.K2_GetActorLocation`) (0.0 0.0 250.0)) (`KismetMathLibrary.MakeRotator` 0.0 0.0 (`KismetMathLibrary.Conv_IntToDouble` (`KismetMathLibrary.FTrunc` (- (`self.SpiralOffset`) 180.0))))) "Undefined" "MultiplyWithRoot" self (stale `SpiralFire` Speed) 0.0 null false 2000.0 (stale `SpiralFire` Damage) (0.0 0.0 0.0) 1.75 self)
  (`|SpawnActorFromClass` "/Game/Projectiles/BP_ProjectileCorona.BP_ProjectileCorona_C" (`KismetMathLibrary.MakeTransform` (- (`self.K2_GetActorLocation`) (0.0 0.0 250.0)) (`KismetMathLibrary.MakeRotator` 0.0 0.0 (`KismetMathLibrary.Conv_IntToDouble` (`KismetMathLibrary.FTrunc` (- (`self.SpiralOffset`) 240.0))))) "Undefined" "MultiplyWithRoot" self (stale `SpiralFire` Speed) 0.0 null false 2000.0 (stale `SpiralFire` Damage) (0.0 0.0 0.0) 1.75 self)
  (`|SpawnActorFromClass` "/Game/Projectiles/BP_ProjectileCorona.BP_ProjectileCorona_C" (`KismetMathLibrary.MakeTransform` (- (`self.K2_GetActorLocation`) (0.0 0.0 250.0)) (`KismetMathLibrary.MakeRotator` 0.0 0.0 (`KismetMathLibrary.Conv_IntToDouble` (`KismetMathLibrary.FTrunc` (- (`self.SpiralOffset`) 300.0))))) "Undefined" "MultiplyWithRoot" self (stale `SpiralFire` Speed) 0.0 null false 2000.0 (stale `SpiralFire` Damage) (0.0 0.0 0.0) 1.75 self)
  (bind _output_get (set `self.SpiralOffset` (+ (`self.SpiralOffset`) 5.0)))
  (if (>= _output_get 360.0)
    (set `self.SpiralOffset` 2.5)))

(event `SpiralFire`
  (params (Duration :type "Float (double-precision)") (Damage :type "Float (double-precision)") (Speed :type "Float (double-precision)"))
  (bind _returnvalue (`KismetSystemLibrary.K2_SetTimerDelegate` (delegate `SpiralSpurt`) 0.05 true))
  (`KismetSystemLibrary.K2_SetTimerDelegate` (delegate `SpirallingWaveBurstEnd`) Duration))

(event `SpirallingWaveBurstEnd`
  (`KismetSystemLibrary.K2_ClearAndInvalidateTimerHandle` (stale `SpiralFire` _returnvalue)))

(event `self.ReceiveTick`
  (params (DeltaSeconds :type "Float (single-precision)"))
  (bind (_returnvalue_roll _returnvalue_pitch _returnvalue_yaw) (`KismetMathLibrary.BreakRotator` (`KismetMathLibrary.FindLookAtRotation` (`SceneComponent.K2_GetComponentLocation` (`self.CapsuleComponent`)) (`CharacterMovementComponent.GetLastUpdateLocation` (`Character.CharacterMovement` (`GameplayStatics.GetPlayerCharacter` 0))))))
  (`self.K2_SetActorRotation` (`KismetMathLibrary.MakeRotator` _returnvalue_roll 0.0 _returnvalue_yaw)))

(event `self.HealthComponent.OnDamageTaken`
  (`GameplayStatics.PlaySoundAtLocation` "/Engine/StarterContent/Audio/MetalClang01.MetalClang01" (`SceneComponent.K2_GetComponentLocation` (`self.CapsuleComponent`)) (struct) 0.01 1.0 0.0 null null null null))

(event `self.CapsuleComponent.OnComponentHit`
  (params (HitComponent :type "PrimitiveComponent Object Reference") (OtherActor :type "Actor Object Reference") (OtherComp :type "PrimitiveComponent Object Reference") (NormalImpulse :type "Vector Structure") (Hit :type "HitResult Structure (by ref)"))
  (bind _returnvalue (`self.GetComponentByClass` OtherActor "/Game/Characters/ActorComponents/HealthComponent.HealthComponent_C"))
  (`/Engine/EditorBlueprintResources/StandardMacros.IsValid` _returnvalue
    (:`Is Valid`
      (`/Game/Characters/ActorComponents/HealthComponent.TakeDamage` _returnvalue 50000.0))))

(event `ChargeAttack`
  (params (Speed :type "Float (double-precision)"))
  (bind _returnvalue (`CharacterMovementComponent.GetLastUpdateLocation` (`Character.CharacterMovement` (`GameplayStatics.GetPlayerCharacter` 0))))
  (bind _returnvalue_2 (`SceneComponent.K2_GetComponentLocation` (`self.CapsuleComponent`)))
  (`self.LaunchCharacter` (* (`KismetMathLibrary.GetDirectionUnitVector` _returnvalue_2 _returnvalue) Speed))
  (`KismetSystemLibrary.Delay` (* (/ (`KismetMathLibrary.Vector_Distance` _returnvalue _returnvalue_2) Speed) 1.25))
  (`MovementComponent.StopMovementImmediately` (`self.CharacterMovement`))
  (`self.RadialBurst` 1500.0 50.0))

(event `BossFightLoop`
  (`self.SpiralFire` 14.4 10.0 750.0)
  (`KismetSystemLibrary.Delay` 15.4)
  (`self.RadialBurst` 1500.0 10.0)
  (`KismetSystemLibrary.Delay` 0.4)
  (`self.RadialBurst` 1500.0 10.0)
  (`KismetSystemLibrary.Delay` 0.8)
  (`self.RadialBurst` 1500.0 10.0)
  (`KismetSystemLibrary.Delay` 0.4)
  (`self.RadialBurst` 1500.0 100.0)
  (`GameplayStatics.PlaySoundAtLocation` "/Engine/StarterContent/Audio/PowerSurge.PowerSurge" (`SceneComponent.K2_GetComponentLocation` (`self.CapsuleComponent`)) (struct) 1.0 1.0 0.0 null null null null)
  (`KismetSystemLibrary.Delay` 2.8)
  (`GameplayStatics.PlaySoundAtLocation` "/Engine/StarterContent/Audio/Sci-Fi_Explosion.Sci-Fi_Explosion" (`SceneComponent.K2_GetComponentLocation` (`self.CapsuleComponent`)) (struct) 1.0 1.0 0.0 null null null null)
  (`self.ChargeAttack` 7500.0)
  (`self.HomingSpray` 50)
  (`KismetSystemLibrary.Delay` 25.0)
  (if (<= (`/Game/Characters/ActorComponents/HealthComponent.Health` (`self.HealthComponent`)) 0.0)
    (`self.K2_DestroyActor`)
    (else
      (`self.BossFightLoop`))))

(event `SpawnHoming`
  (`|SpawnActorFromClass` "/Game/Projectiles/BP_ProjectileCorona.BP_ProjectileCorona_C" (`KismetMathLibrary.MakeTransform` (+ (`self.K2_GetActorLocation`) (0.0 0.0 300.0)) (`KismetMathLibrary.MakeRotator` 0.0 0.0 90.0)) "Undefined" "MultiplyWithRoot" self 1500.0 0.0 (`GameplayStatics.GetPlayerCharacter` 0) true 2000.0 10.0 (0.0 0.0 0.0) (`KismetMathLibrary.Conv_IntToDouble` (/ (stale `HomingSpray` Number) 2)) self))

(event `HomingSpray`
  (params (Number :type Integer))
  (bind _returnvalue (`KismetSystemLibrary.K2_SetTimerDelegate` (delegate `SpawnHoming`) 0.5 true))
  (`KismetSystemLibrary.K2_SetTimerDelegate` (delegate `EndHomingSpray`) (`KismetMathLibrary.Conv_IntToDouble` (/ Number 2))))

(event `self.ReceiveBeginPlay`
  (`self.BossFightLoop`))

(event `EndHomingSpray`
  (`KismetSystemLibrary.K2_ClearAndInvalidateTimerHandle` (stale `HomingSpray` _returnvalue)))

(fn `UserConstructionScript`)